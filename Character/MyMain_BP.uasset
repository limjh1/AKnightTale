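; Player character Blueprint with four mana-and-cooldown abilities: heal, thrown knife, mana restore and super attack, the last two gated by Level.
; Casts lock movement and exclude each other via Casting flags; cooldowns refill through Delay loops.
; Tick regenerates Health and Mana and handles skill unlocks, with one-time Quest messages sent to CritterGameMode_BP.
; Other inputs handle a launch-based dash, inventory, save/load, pickup display and game-over widget.
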(event EventBeginPlay)

(event Collision|EventActorBeginOverlap
  (params (OtherActor :type Actor%20Object%20Reference)))

(event EventTick
  (params (DeltaSeconds :type Float%20%28single-precision%29))
  (Utilities|FlowControl|Sequence
    (:then_0
      ;[1 0.6094 0.6094] HealthRegen
      (Utilities|FlowControl|Delay (Variables|Default|GetHealthRate))
      (if (< (Variables|Default|GetHealth) 1e+02)
        (Variables|Default|SetHealth (+ (Variables|Default|GetHealth) (Variables|Default|GetHealthRegen)))
        (if (> (Variables|Default|GetHealth) 1e+02)
          (Variables|Default|SetHealth 1e+02))))
    (:then_1
      ;[0.6719 0.6968 1] ManaRegen
      (Utilities|FlowControl|Delay (Variables|Default|GetManaRate))
      (if (< (Variables|Default|GetMana) 1e+02)
        (Variables|Default|SetMana (+ (Variables|Default|GetMana) (Variables|Default|GetManaRegen)))
        (if (> (Variables|Default|GetMana) 1e+02)
          (Variables|Default|SetMana 1e+02))))
    (:then_2
      (if (>= (Variables|Default|GetLevel) 2)
        (Utilities|FlowControl|DoOnce false
          (:Completed
            (bind _ascritter_game_mode_bp (Utilities|Casting|CastToCritterGameMode_BP (Game|GetGameMode)))
            (Variables|/Game/Blueprints/CritterGameMode_BP.CritterGameMode_BP_C|SetQuest _ascritter_game_mode_bp "3번 스킬을 획득하였습니다. 사용해보세요.")
            (Variables|Default|SetSkill3CoolDown 1.0)))
        (else
          (Variables|Default|SetSkill3CoolDown 0.0))))
    (:then_3
      (if (>= (Variables|Default|GetLevel) 3)
        (Utilities|FlowControl|DoOnce false
          (:Completed
            (bind _ascritter_game_mode_bp_2 (Utilities|Casting|CastToCritterGameMode_BP (Game|GetGameMode)))
            (Variables|/Game/Blueprints/CritterGameMode_BP.CritterGameMode_BP_C|SetQuest _ascritter_game_mode_bp_2 "4번 스킬을 획득하였습니다. 사용해보세요.")
            (Variables|Default|SetSkill4CoolDown 1.0)))
        (else
          (Variables|Default|SetSkill4CoolDown 0.0))))))

(event Input|ActionEvents|InputActionAbility1
  (params (Key :type Key%20Structure :default "None"))
  (bind _charactermovement (Variables|Character|GetCharacterMovement))
  (:Pressed
    (Utilities|FlowControl|Sequence
      (:then_0
        (Utilities|FlowControl|DoOnce false
          (:Completed
            (bind _ascritter_game_mode_bp (Utilities|Casting|CastToCritterGameMode_BP (Game|GetGameMode)))
            (Variables|/Game/Blueprints/CritterGameMode_BP.CritterGameMode_BP_C|SetQuest _ascritter_game_mode_bp "체력이 회복됩니다. 2번을 눌러주세요."))))
      (:then_1
        (if (>= (Variables|Default|GetSkill1CoolDown) 1.0)
          (if (not (Math|Boolean|ORBoolean (Variables|Default|GetCastingHeal) (Variables|Default|GetCasting%20Knife) (Variables|Default|GetCastingMana) (Variables|Default|GetCastingSuperAtk)))
            (if (< (Variables|Default|GetMana) 15.0)
              (bind _returnvalue (UserInterface|CreateWidget "/Game/Blueprints/NoManaPopup.NoManaPopup_C"))
              (UserInterface|Viewport|AddtoViewport _returnvalue 0)
              (elif (not (>= (Variables|Default|GetHealth) 1e+02))
                (Variables|Default|SetCastingHeal true)
                (Pawn|Components|CharacterMovement|DisableMovement _charactermovement)
                (Components|Movement|StopMovementImmediately _charactermovement)
                (Variables|Default|SetHealth (+ (Variables|Default|GetHealth) 25.0))
                (Variables|Default|SetMana (- (Variables|Default|GetMana) 15.0))
                (Effects|SpawnEmitteratLocation "/Game/InfinityBladeEffects/Effects/FX_Ability/Heal/P_Heal_LongDistance_Start.P_Heal_LongDistance_Start" (Transformation|GetSocketLocation (Variables|Character|GetMesh) "RightFoot"))
                (Audio|PlaySound2D "/Game/HumanVocalizations/HumanFemaleA/Cues/voice_female_a_growl_03_Cue.voice_female_a_growl_03_Cue" 1.0 1.0 0.0 0 0)
                (Utilities|FlowControl|Delay 1.0)
                (Pawn|Components|CharacterMovement|SetMovementMode (Variables|Character|GetCharacterMovement) "MOVE_Walking" 0)
                (Variables|Default|SetCastingHeal false)
                (Variables|Default|SetSkill1CoolDown 0.0)
                (if (< (Variables|Default|GetSkill1CoolDown) 1.0) :!label _label
                  (Variables|Default|SetSkill1CoolDown (+ (Variables|Default|GetSkill1CoolDown) 0.025))
                  (Utilities|FlowControl|Delay 0.1)
                  (goto _label))))))))))

(event Input|ActionEvents|InputActionOpenBag
  (params (Key :type Key%20Structure :default "None"))
  (:Pressed
    (bind _returnvalue (UserInterface|CreateWidget "/Game/HUD/Inventory.Inventory_C"))
    (if (Variables|Default|GetbagTrue)
      (UserInterface|Viewport|AddtoViewport _returnvalue 0)
      (bind _asplayer_controller (Utilities|Casting|CastToPlayerController (Game|GetPlayerController 0)))
      (Variables|/Script/Engine.PlayerController|SetbShowMouseCursor _asplayer_controller true)
      (Variables|Default|SetbagTrue false)
      (Utilities|FlowControl|Delay 1.0))
    (bind _asplayer_controller_2 (Utilities|Casting|CastToPlayerController (Game|GetPlayerController 0)))
    (Variables|/Script/Engine.PlayerController|SetbShowMouseCursor _asplayer_controller_2 false)
    (Variables|Default|SetbagTrue true)
    (Widget|RemovefromParent _returnvalue)))

(event Input|ActionEvents|InputActionAbility3
  (params (Key :type Key%20Structure :default "None"))
  (bind _charactermovement (Variables|Character|GetCharacterMovement))
  (:Pressed
    (if (>= (Variables|Default|GetLevel) 2)
      (Utilities|FlowControl|Sequence
        (:then_0
          (Utilities|FlowControl|DoOnce false
            (:Completed
              (bind _ascritter_game_mode_bp (Utilities|Casting|CastToCritterGameMode_BP (Game|GetGameMode)))
              (Variables|/Game/Blueprints/CritterGameMode_BP.CritterGameMode_BP_C|SetQuest _ascritter_game_mode_bp "마나를 회복합니다. 계속해서 레벨을 올려주세요."))))
        (:then_1
          (if (>= (Variables|Default|GetSkill3CoolDown) 1.0)
            (if (not (Math|Boolean|ORBoolean (Variables|Default|GetCastingHeal) (Variables|Default|GetCasting%20Knife) (Variables|Default|GetCastingMana) (Variables|Default|GetCastingSuperAtk)))
              (if (not (>= (Variables|Default|GetMana) 1e+02))
                (Variables|Default|SetCastingMana true)
                (Pawn|Components|CharacterMovement|DisableMovement _charactermovement)
                (Components|Movement|StopMovementImmediately _charactermovement)
                (Variables|Default|SetMana (+ (Variables|Default|GetMana) 1e+02))
                (if (> (Variables|Default|GetMana) 1e+02)
                  (Variables|Default|SetMana 1e+02))
                (Utilities|FlowControl|Delay 0.4)
                (Effects|SpawnEmitteratLocation "/Game/InfinityBladeEffects/Effects/FX_Ability/Summon/HealEffects.HealEffects" (Transformation|GetSocketLocation (Variables|Character|GetMesh) "RightFoot"))
                (Audio|PlaySound2D "/Game/HumanVocalizations/HumanFemaleA/Wavs/voice_female_a_growl_06.voice_female_a_growl_06" 1.0 1.0 0.0 0 0)
                (Utilities|FlowControl|Delay 1.3)
                (Pawn|Components|CharacterMovement|SetMovementMode (Variables|Character|GetCharacterMovement) "MOVE_Walking" 0)
                (Variables|Default|SetCastingMana false)
                (Variables|Default|SetSkill3CoolDown 0.0)
                (if (< (Variables|Default|GetSkill3CoolDown) 1.0) :!label _label
                  (Variables|Default|SetSkill3CoolDown (+ (Variables|Default|GetSkill3CoolDown) 0.025))
                  (Utilities|FlowControl|Delay 0.5)
                  (goto _label))))))))))

(event Input|ActionEvents|InputActionAbility2
  (params (Key :type Key%20Structure :default "None"))
  (bind _charactermovement (Variables|Character|GetCharacterMovement))
  (:Pressed
    (Utilities|FlowControl|Sequence
      (:then_0
        (Utilities|FlowControl|DoOnce false
          (:Completed
            (bind _ascritter_game_mode_bp (Utilities|Casting|CastToCritterGameMode_BP (Game|GetGameMode)))
            (Variables|/Game/Blueprints/CritterGameMode_BP.CritterGameMode_BP_C|SetQuest _ascritter_game_mode_bp "단검을 던집니다. 이제 몬스터 찾아주세요.."))))
      (:then_1
        (if (>= (Variables|Default|GetSkill2CoolDown) 1.0)
          (if (not (Math|Boolean|ORBoolean (Variables|Default|GetCastingHeal) (Variables|Default|GetCasting%20Knife) (Variables|Default|GetCastingMana) (Variables|Default|GetCastingSuperAtk)))
            (if (< (Variables|Default|GetMana) 15.0)
              (bind _returnvalue (UserInterface|CreateWidget "/Game/Blueprints/NoManaPopup.NoManaPopup_C"))
              (UserInterface|Viewport|AddtoViewport _returnvalue 0)
              (else
                (Variables|Default|SetCasting%20Knife true)
                (Pawn|Components|CharacterMovement|DisableMovement _charactermovement)
                (Components|Movement|StopMovementImmediately _charactermovement)
                (Variables|Default|SetMana (- (Variables|Default|GetMana) 15.0))
                (Utilities|FlowControl|Delay 0.4)
                (Effects|SpawnEmitteratLocation "/Game/InfinityBladeEffects/Effects/FX_Combat_Base/death/P_Impact_Gib_Ice.P_Impact_Gib_Ice" (Transformation|GetSocketLocation (Variables|Character|GetMesh) "RightFoot"))
                (Game|SpawnActorfromClass "/Game/Character/ThrowKnfie.ThrowKnfie_C" (Math|Transform|MakeTransform (Transformation|GetSocketLocation (Variables|Character|GetMesh) "LeftHand") (Transformation|GetActorRotation) (Transformation|GetActorScale3D)) "Undefined" 0 0)
                (Audio|PlaySound2D "/Game/HumanVocalizations/HumanFemaleA/Wavs/voice_female_a_attack_02.voice_female_a_attack_02" 1.0 1.0 0.0 0 0)
                (Utilities|FlowControl|Delay 0.8)
                (Pawn|Components|CharacterMovement|SetMovementMode (Variables|Character|GetCharacterMovement) "MOVE_Walking" 0)
                (Variables|Default|SetCasting%20Knife false)
                (Variables|Default|SetSkill2CoolDown 0.0)
                (if (< (Variables|Default|GetSkill2CoolDown) 1.0) :!label _label
                  (Variables|Default|SetSkill2CoolDown (+ (Variables|Default|GetSkill2CoolDown) 0.025))
                  (Utilities|FlowControl|Delay 0.05)
                  (goto _label))))))))))

(event Input|ActionEvents|InputActionAbility4
  (params (Key :type Key%20Structure :default "None"))
  (bind _charactermovement (Variables|Character|GetCharacterMovement))
  (:Pressed
    (if (>= (Variables|Default|GetLevel) 3)
      (Utilities|FlowControl|Sequence
        (:then_0
          (Utilities|FlowControl|DoOnce false
            (:Completed
              (bind _ascritter_game_mode_bp (Utilities|Casting|CastToCritterGameMode_BP (Game|GetGameMode)))
              (Variables|/Game/Blueprints/CritterGameMode_BP.CritterGameMode_BP_C|SetQuest _ascritter_game_mode_bp "강력한 에너지를 던집니다. 이제 보스 몬스터를 찾아 사냥해주세요!"))))
        (:then_1
          (if (>= (Variables|Default|GetSkill4CoolDown) 1.0)
            (if (not (Math|Boolean|ORBoolean (Variables|Default|GetCastingHeal) (Variables|Default|GetCasting%20Knife) (Variables|Default|GetCastingMana) (Variables|Default|GetCastingSuperAtk)))
              (if (< (Variables|Default|GetMana) 5e+01)
                (bind _returnvalue (UserInterface|CreateWidget "/Game/Blueprints/NoManaPopup.NoManaPopup_C"))
                (UserInterface|Viewport|AddtoViewport _returnvalue 0)
                (else
                  (Variables|Default|SetCastingSuperAtk true)
                  (Pawn|Components|CharacterMovement|DisableMovement _charactermovement)
                  (Components|Movement|StopMovementImmediately _charactermovement)
                  (Variables|Default|SetMana (- (Variables|Default|GetMana) 5e+01))
                  (Effects|SpawnEmitteratLocation "/Game/InfinityBladeEffects/Effects/FX_Skill_TeleCharge/P_Skill_Telecharge_Ice_Impact_03.P_Skill_Telecharge_Ice_Impact_03" (Transformation|GetSocketLocation (Variables|Character|GetMesh) "FootMid"))
                  (Utilities|FlowControl|Delay 0.9)
                  (Game|SpawnActorfromClass "/Game/Character/SuperAtk.SuperAtk_C" (Math|Transform|MakeTransform (Transformation|GetSocketLocation (Variables|Character|GetMesh) "HeadAtk") (Transformation|GetActorRotation) (Transformation|GetActorScale3D)) "Undefined" 0 0)
                  (Audio|PlaySound2D "/Game/HumanVocalizations/HumanFemaleA/Cues/voice_female_a_battle_shout_01_Cue.voice_female_a_battle_shout_01_Cue" 1.0 1.0 0.0 0 0)
                  (Utilities|FlowControl|Delay 1.3)
                  (Pawn|Components|CharacterMovement|SetMovementMode (Variables|Character|GetCharacterMovement) "MOVE_Walking" 0)
                  (Variables|Default|SetCastingSuperAtk false)
                  (Variables|Default|SetSkill4CoolDown 0.0)
                  (if (< (Variables|Default|GetSkill4CoolDown) 1.0) :!label _label
                    (Variables|Default|SetSkill4CoolDown (+ (Variables|Default|GetSkill4CoolDown) 0.025))
                    (Utilities|FlowControl|Delay 0.2)
                    (goto _label)))))))))))

(event Input|KeyboardEvents|R
  (params (Key :type Key%20Structure :default "None"))
  (:Pressed
    (Class|Main|SaveGame)))

(event Input|KeyboardEvents|N
  (params (Key :type Key%20Structure :default "None"))
  (:Pressed
    (Class|Main|ShowPickupLocations)))

(event Input|KeyboardEvents|T
  (params (Key :type Key%20Structure :default "None"))
  (:Pressed
    (Class|Main|LoadGame true)))

(event Input|KeyboardEvents|Enter
  (params (Key :type Key%20Structure :default "None"))
  (:Pressed
    (bind _returnvalue (UserInterface|CreateWidget "/Game/HUD/UI_GameOver.UI_GameOver_C"))
    (UserInterface|Viewport|AddtoViewport _returnvalue 0)))

(event Input|KeyboardEvents|E
  (params (Key :type Key%20Structure :default "None"))
  (bind _returnvalue (Game|GetPlayerController 0))
  (:Pressed
    (if (Math|Boolean|ORBoolean (Game|Player|IsInputKeyDown _returnvalue "W") (Game|Player|IsInputKeyDown _returnvalue "A") (Game|Player|IsInputKeyDown _returnvalue "S") (Game|Player|IsInputKeyDown _returnvalue "D"))
      (Utilities|FlowControl|DoOnce false :!label _label
        (:Completed
          (Character|LaunchCharacter "0, 0,200.000000" false false)
          (Utilities|FlowControl|Delay 0.1)
          (Character|LaunchCharacter (* (Math|Vector|GetForwardVector (Transformation|GetActorRotation)) 1e+03) false false)
          (Utilities|FlowControl|Delay 1.0)
          (goto _label Reset))))))

(fn ConstructionScript)